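; BP_BotSpawner fills Mordhau matches with bots, adapting to the game mode detected at BeginPlay.
; A delayed loop adds batches while enough players are present and the match has started (not required for Skirmish), otherwise clearing all bots and restarting.
; Team 0 always receives bots, while team 1 is skipped for modes like Horde and Battle Royale.
; The per-team target is compared against batches spawned, not individual bots.
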(event EventBeginPlay
  (bind _returnvalue (Game|GetGameMode))
  (bind _botspawnerbotbatchsize (Variables|Default|GetbotSpawnerBotBatchSize))
  (bind _asmordhau_game_mode (Utilities|Casting|CastToMordhauGameMode _returnvalue))
  (Utilities|Casting|CastToBP_SkirmishGameMode _returnvalue
    (:then
      (Variables|Default|SetlocalMatchType "NewEnumerator0"))
    (:CastFailed
      (Utilities|Casting|CastToBP_HordeGameMode _returnvalue
        (:then
          (Variables|Default|SetlocalMatchType "NewEnumerator1"))
        (:CastFailed
          (Utilities|Casting|CastToBP_BattleRoyaleGameMode _returnvalue
            (:then
              (Variables|Default|SetlocalMatchType "NewEnumerator4"))
            (:CastFailed
              (Utilities|Casting|CastToBP_FrontlineGameMode _returnvalue
                (:then
                  (Variables|Default|SetlocalMatchType "NewEnumerator3"))
                (:CastFailed
                  (Utilities|Casting|CastToBP_TeamDeathmatchGameMode _returnvalue
                    (:then
                      (Variables|Default|SetlocalMatchType "NewEnumerator5"))
                    (:CastFailed
                      _))))))))))
  (Class|MordhauGameMode|RemoveBots _asmordhau_game_mode 1000 :!label _label)
  (Class|MordhauGameMode|RemoveBots _asmordhau_game_mode 1000 1)
  (Variables|Default|SetlocalNumBots 0)
  (Utilities|FlowControl|Delay (Variables|Default|GetbotSpawnerInitialDelaySeconds))
  (bind _returnvalue_2 (Class|GameModeBase|GetNumPlayers _returnvalue :!label _label_2))
  (if (and (or (Utilities|Enum|Equal(Enum) (Variables|Default|GetlocalMatchType) "NewEnumerator0") (Class|GameModeBase|HasMatchStarted _returnvalue)) (>= _returnvalue_2 (Variables|Default|GetbotSpawnerMinimumPlayers)))
    (if (< (Variables|Default|GetlocalNumBots) (Variables|Default|GetbotSpawnerTargetBotsPerTeam))
      (Class|MordhauGameMode|AddBots _asmordhau_game_mode _botspawnerbotbatchsize)
      (if (Math|Boolean|ANDBoolean (Utilities|Enum|NotEqual(Enum) (Variables|Default|GetlocalMatchType) "NewEnumerator1") (Utilities|Enum|NotEqual(Enum) (Variables|Default|GetlocalMatchType) "NewEnumerator4") (Utilities|Enum|NotEqual(Enum) (Variables|Default|GetlocalMatchType) "NewEnumerator2"))
        (Class|MordhauGameMode|AddBots _asmordhau_game_mode _botspawnerbotbatchsize 1))
      (Math|Integer|IncrementInt (Variables|Default|GetlocalNumBots)
        (:%20%20
          _)))
    (Utilities|FlowControl|Delay (Variables|Default|GetbotSpawnerSpawnDelaySeconds))
    (goto _label_2)
    (else
      (goto _label))))

(event Collision|EventActorBeginOverlap
  (params (OtherActor :type Actor%20Object%20Reference)))

(event EventTick
  (params (DeltaSeconds :type Float%20%28single-precision%29)))

(fn ConstructionScript)